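; Cat character that follows the player and plays a looping double-attack montage at close range, then destroys itself after a 30-second lifetime.
; Tick refreshes distance and direction to the player, then drives an Idle, Follow Char and Attack state machine using distance thresholds.
; OnAnimEnd_Attack either replays the montage or resumes following.
; Tick also pulses a Plane's scale, growing it on odd seconds and resetting it on even ones.
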(event Custom|OnAnimEnd_Attack
  (Variables|Default|SetIs%20Attacking false)
  (if (> (Variables|Default|GetDistance%20Player%20Character) 1e+02)
    (Variables|Default|SetCurState "NewEnumerator1")
    (else
      (Animation|PlayAnimMontage "/Game/LowPoly_Cat/Animations/Anim_Cat_Attack_Double_Montage.Anim_Cat_Attack_Double_Montage" 1.0 "None")
      (Variables|Default|SetIs%20Attacking true))))

(event EventBeginPlay)

(event EventTick
  (params (DeltaSeconds :type Float%20%28single-precision%29))
  (bind _plane (Variables|Default|GetPlane))
  (Variables|Default|Settime (+ DeltaSeconds (Variables|Default|Gettime)))
  (Utilities|FlowControl|Sequence
    (:then_0
      ;[1 1 1] 코멘트
      (if (< (Variables|Default|Gettime) 3e+01)
        (CallFunction|SaveDistandDir)
        (switch Utilities|FlowControl|Switch|SwitchonCat01State (Variables|Default|GetCurState)
          (:NewEnumerator0
            (if (<= (Variables|Default|GetDistance%20Player%20Character) 3e+02)
              (Variables|Default|SetCurState "NewEnumerator1")))
          (:NewEnumerator1
            (if (<= (Variables|Default|GetDistance%20Player%20Character) 9e+01)
              (Variables|Default|SetCurState "NewEnumerator2")
              (Animation|PlayAnimMontage "/Game/LowPoly_Cat/Animations/Anim_Cat_Attack_Double_Montage.Anim_Cat_Attack_Double_Montage" 1.0 "None")
              (Variables|Default|SetIs%20Attacking true)
              (else
                (Pawn|Input|AddMovementInput (Variables|Default|GetDirToPlayerCharacter) 1.0 false))))
          (:NewEnumerator2
            (if (Variables|Default|GetIs%20Attacking)
              (if (> (Variables|Default|GetDistance%20Player%20Character) 1e+02)
                (Variables|Default|SetCurState "NewEnumerator1")))))
        (else
          (Actor|DestroyActor))))
    (:then_1
      (if (== (Math|Integer|%(Integer) (Math|Float|Truncate (Variables|Default|Gettime)) 2) 0)
        (Transformation|SetWorldScale3D (Variables|Default|GetPlane) "1.000000,1.000000,1.000000")
        (else
          (Transformation|SetWorldScale3D _plane (+ (Transformation|GetWorldScale _plane) (Utilities|Time|GetWorldDeltaSeconds))))))))

(event Collision|EventActorBeginOverlap
  (params (OtherActor :type Actor%20Object%20Reference)))

(fn ConstructionScript)

(fn SaveDistandDir
  (bind _returnvalue (Game|GetPlayerCharacter 0))
  (bind _returnvalue_2 (Transformation|GetActorLocation))
  (bind _returnvalue_3 (Transformation|GetActorLocation _returnvalue))
  (bind _returnvalue_4 (- _returnvalue_3 _returnvalue_2))
  (bind (_x _y _z) (Math|Vector|BreakVector _returnvalue_4))
  (bind _returnvalue_5 (Math|Vector|MakeVector _x _y _z))
  (Variables|Default|SetDistance%20Player%20Character (Math|Vector|VectorLength _returnvalue_5))
  (Variables|Default|SetDirToPlayerCharacter (Math|Vector|Normalize _returnvalue_5)))