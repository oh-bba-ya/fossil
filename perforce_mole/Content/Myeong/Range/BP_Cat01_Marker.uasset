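; BP_Cat01_Marker is a marker actor that hovers above a Cat01BP actor with a repeating grow-and-reset pulse.
; Each Tick it fetches all Cat01BP actors again and places the Marker component just above the one at array index 1, with no bounds check.
; Delta time steadily enlarges the marker's scale until a two-second timer expires, resetting both timer and scale.
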(event EventBeginPlay)

(event Collision|EventActorBeginOverlap
  (params (OtherActor :type Actor%20Object%20Reference)))

(event EventTick
  (params (DeltaSeconds :type Float%20%28single-precision%29))
  (bind _marker (Variables|Default|GetMarker))
  (Variables|Default|Settime (+ DeltaSeconds (Variables|Default|Gettime)))
  (if (> (Variables|Default|Gettime) 2.0)
    (Variables|Default|Settime 0.0)
    (Transformation|SetWorldScale3D (Variables|Default|GetMarker) "1.000000,1.000000,1.000000")
    (else
      (bind _outactors (Actor|GetAllActorsOfClass "/Game/Myeong/Range/Cat01BP.Cat01BP_C"))
      (bind _output_get (Variables|디폴트|SetCat_Loc _outactors))
      (Transformation|SetWorldLocation _marker (+ (Transformation|GetWorldLocation (Variables|/Script/Engine.Actor|GetRootComponent (Utilities|Array|Get(acopy) _output_get 1))) "0.000000,0.000000,100.000000") false false)
      (Transformation|SetWorldScale3D _marker (+ (Transformation|GetWorldScale _marker) (Utilities|Time|GetWorldDeltaSeconds))))))

(fn ConstructionScript)