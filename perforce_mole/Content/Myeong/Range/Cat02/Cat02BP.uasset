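; Cat enemy character with a Tick-driven Idle, Follow and Attack state machine that chases and claws the player.
; It follows when the player is near and above zero Z, steers toward its spawn point when out of range, and repeats an attack montage up close.
; Attack events toggle both hit colliders, though only the left one applies damage.
; A Marker event pulses a plane's scale over time.
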(event OnComponentBeginOverlap(LeftCollision)
  (params (OverlappedComponent :type Primitive%20Component%20Object%20Reference) (OtherActor :type Actor%20Object%20Reference) (OtherComp :type Primitive%20Component%20Object%20Reference) (OtherBodyIndex :type Integer) (bFromSweep :type Boolean) (SweepResult :type Hit%20Result%20Structure%20%28by%20ref%29))
  (if (!= OtherActor self)
    (Game|Damage|ApplyDamage OtherActor (Variables|Default|GetAtk) 0 self)))

(event Custom|SaveDisAndDir
  (bind _output_get (Variables|Default|SetPlayerPos (Transformation|GetActorLocation (Game|GetPlayerCharacter 0))))
  (Variables|Default|SetDistancePlayerChar (Math|Vector|VectorLength (- _output_get (Transformation|GetActorLocation))))
  (Variables|Default|SetDirToPlayerChar (Math|Vector|Normalize (- _output_get (Transformation|GetActorLocation)))))

(event Custom|OnColEnd_Attack
  (Collision|SetCollisionEnabled (Variables|Default|GetRightCollision) "NoCollision")
  (Collision|SetCollisionEnabled (Variables|Default|GetLeftCollision) "NoCollision"))

(event Custom|Marker
  (bind _plane (Variables|Default|GetPlane))
  (Variables|Default|SetTime (+ (Utilities|Time|GetWorldDeltaSeconds) (Variables|Default|GetTime)))
  (if (== (Math|Integer|%(Integer) (Math|Float|Truncate (Variables|Default|GetTime)) 2) 0)
    (Transformation|SetWorldScale3D (Variables|Default|GetPlane) "1.000000,1.000000,1.000000")
    (else
      (Transformation|SetWorldScale3D _plane (+ (Transformation|GetWorldScale _plane) (Utilities|Time|GetWorldDeltaSeconds))))))

(event Custom|OnColStart_Attack
  (Collision|SetCollisionEnabled (Variables|Default|GetRightCollision) "QueryAndPhysics")
  (Collision|SetCollisionEnabled (Variables|Default|GetLeftCollision) "QueryAndPhysics"))

(event Custom|BackPosition
  (bind _output_get (Variables|Default|SetoriginalPos (Variables|Default|GetoriginalPos)))
  (Variables|Default|SetDirToOriginalPos (Math|Vector|Normalize (- _output_get (Transformation|GetActorLocation)))))

(event Custom|OnAnimEnd_Attack
  (Variables|Default|SetIsAttacking false)
  (if (> (Variables|Default|GetDistancePlayerChar) 1.8e+02)
    (Variables|Default|SetCurState "NewEnumerator1")
    (else
      (Animation|PlayAnimMontage "/Game/LowPoly_Cat/Animations/Anim_Cat_Attack_Double_Montage1.Anim_Cat_Attack_Double_Montage1" 1.0 "None")
      (Variables|Default|SetIsAttacking true))))

(event EventBeginPlay
  (Variables|Default|SetoriginalPos (Transformation|GetActorLocation)))

(event Collision|EventActorBeginOverlap
  (params (OtherActor :type Actor%20Object%20Reference)))

(event EventTick
  (params (DeltaSeconds :type Float%20%28single-precision%29))
  (CallFunction|BackPosition)
  (CallFunction|Marker)
  (CallFunction|SaveDisandDir)
  (switch Utilities|FlowControl|Switch|SwitchonCat02State (Variables|Default|GetCurState)
    (:NewEnumerator0
      (if (<= (Variables|Default|GetDistancePlayerChar) 5e+02)
        (if (> (.Z (Math|Vector|BreakVector (Variables|Default|GetPlayerPos))) 0.0)
          (Audio|PlaySound2D "/Game/Myeong/Sound/CatSound.CatSound" 0.05 1.0 0.0 0 0)
          (Variables|Default|SetCurState "NewEnumerator1")
          (else
            (Variables|Default|SetCurState "NewEnumerator0")))
        (else
          (Variables|Default|SetCurState "NewEnumerator0"))))
    (:NewEnumerator1
      (if (<= (Variables|Default|GetDistancePlayerChar) 5e+02)
        (if (> (.Z (Math|Vector|BreakVector (Variables|Default|GetPlayerPos))) 0.0)
          (Pawn|Input|AddMovementInput (Variables|Default|GetDirToPlayerChar) 1.0 false)
          (if (<= (Variables|Default|GetDistancePlayerChar) 1.6e+02)
            (Variables|Default|SetCurState "NewEnumerator2")
            (Animation|PlayAnimMontage "/Game/LowPoly_Cat/Animations/Anim_Cat_Attack_Double_Montage1.Anim_Cat_Attack_Double_Montage1" 1.0 "None")
            (Variables|Default|SetIsAttacking true))
          (else
            (Variables|Default|SetCurState "NewEnumerator0")))
        (else
          (Pawn|Input|AddMovementInput (Variables|Default|GetDirToOriginalPos) 1.0 false))))
    (:NewEnumerator2
      (if (not (Variables|Default|GetIsAttacking))
        (if (> (Variables|Default|GetDistancePlayerChar) 1.8e+02)
          (Variables|Default|SetCurState "NewEnumerator1"))))))

(fn ConstructionScript)